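; Soft-body dynamic mesh actor prototype, built from a copied editor sphere with a BVH and complex collision.
; BeginPlay calls SetMeshInfo and Tick runs MeshToSoftBody, whose internals are not in this file.
; Disconnected experiments deform vertices against another mesh through BVH queries.
; The uncalled, unfinished TetGen prepares tetrahedralization points (jittered vertices, grid samples, enclosing tetrahedron), but its IsInside ray test never returns a result.
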(event OnComponentHit(DynamicMeshComponent)
  (params (HitComponent :type Primitive%20Component%20Object%20Reference) (OtherActor :type Actor%20Object%20Reference) (OtherComp :type Primitive%20Component%20Object%20Reference) (NormalImpulse :type Vector :default "0, 0, 0") (Hit :type Hit%20Result%20Structure%20%28by%20ref%29)))

(event EventTick
  (params (DeltaSeconds :type Float%20%28single-precision%29))
  (Class|SoftBody|MeshtoSoftBody (Variables|Default|GetTarget%20Mesh) 0 DeltaSeconds))

(event EventBeginPlay
  (Class|SoftBody|SetMeshInfo (Variables|Default|GetTarget%20Mesh) 0 1e+01))

(event EventOnRebuildSoftBodyMesh
  (params (TargetMesh :type Dynamic%20Mesh%20Object%20Reference))
  (bind _returnvalue (GeometryScript|StaticMesh|CopyMeshFromStaticMesh :FromStaticMeshAsset "/Engine/EditorMeshes/ArcadeEditorSphere.ArcadeEditorSphere" :ToDynamicMesh TargetMesh :Debug 0)
    (:Success
      (bind (_outputbvh _returnvalue_2) (Class|GeometryScriptLibraryMeshSpatial|BuildBVHforMesh _returnvalue 0))
      (Variables|Default|SetOutput%20BVH _outputbvh)
      (bind _returnvalue_3 (Class|GeometryScriptLibraryMeshSubdivideFunctions|ApplyPNTessellation :TargetMesh _returnvalue_2 :TessellationLevel 0 :Debug 0))
      (Variables|Default|SetTarget%20Mesh _returnvalue_3)
      (Class|DynamicMeshComponent|EnableComplexasSimpleCollision (Variables|Default|GetDynamicMeshComponent)))))

(fn ConstructionScript)

(fn TetGen
  (params (DynamicMesh :type Dynamic%20Mesh%20Object%20Reference) (resolution :type Float%20%28double-precision%29))
  (bind _infiniy (Variables|Default|GetInfiniy))
  (bind _tetverts (Variables|Default|GetTetVerts))
  (Variables|Default|SetResolution resolution)
  ;[1 1 1] 1Step
  (bind _positionlist (GeometryScript|MeshQueries|GetAllVertexPositions DynamicMesh))
  (bind _vectorarray (Class|GeometryScriptLibraryListUtilityFunctions|ConvertVectorListtoArray _positionlist))
  (for _array_element _vectorarray
    (bind _eps (CallFunction|RandEps))
    (bind _eps_2 (CallFunction|RandEps))
    (bind _eps_3 (CallFunction|RandEps))
    (Utilities|Array|Add (Variables|Default|GetTetVerts) (Math|Vector|MakeVector (+ (.x _array_element) _eps) (+ (.y _array_element) _eps_2) (+ _eps_3 (.z _array_element)))))
  (Variables|Default|Setbmin _infiniy)
  (Variables|Default|Setbmax (* _infiniy -1.0))
  ;[1 1 1] 2Step
  (for _array_element_2 (Variables|Default|GetTetVerts)
    (bind _output_get (Variables|Default|SetCenter (+ _array_element_2 (Variables|Default|GetCenter))))
    (Variables|Default|Setbmin (Math|Vector|MakeVector (Math|Float|Min(Float) (.x (Variables|Default|Getbmin)) (.x _output_get)) (Math|Float|Min(Float) (.y (Variables|Default|Getbmin)) (.y _output_get)) (Math|Float|Min(Float) (.z (Variables|Default|Getbmin)) (.z _output_get))))
    (Variables|Default|Setbmax (Math|Vector|MakeVector (Math|Float|Max(Float) (.x (Variables|Default|Getbmax)) (.x _output_get)) (Math|Float|Max(Float) (.y (Variables|Default|Getbmax)) (.y _output_get)) (Math|Float|Max(Float) (.z (Variables|Default|Getbmax)) (.z _output_get)))))
  (Variables|Default|SetCenter (/ (Variables|Default|GetCenter) (Utilities|Array|Length (Variables|Default|GetTetVerts))))
  ;[1 1 1] Step3
  (Variables|Default|Setradius 0.0)
  (for _array_element_3 (Variables|Default|GetTetVerts)
    (Variables|Default|Setradius (Math|Float|Max(Float) (Math|Vector|VectorLength (- _array_element_3 (Variables|Default|GetCenter))) (Variables|Default|Getradius))))
  ;[1 1 1] Step4
  (Utilities|FlowControl|Sequence
    (:then_0
      (if (> (Variables|Default|GetResolution) 0.0)
        (Variables|Default|Setdims (- (Variables|Default|Getbmax) (Variables|Default|Getbmin)))
        (bind _output_get_2 (Variables|Default|Setdim (Math|Float|Max(Float) (.x (Variables|Default|Getdims)) (Math|Float|Max(Float) (.y (Variables|Default|Getdims)) (.z (Variables|Default|Getdims))))))
        (Variables|Default|Seth (/ _output_get_2 (Variables|Default|GetResolution)))
        (for _index (range 0 (Math|Conversions|ToInteger(Byte) (/ (.x (Variables|Default|Getdims)) (Variables|Default|Geth))))
          (bind _eps_4 (CallFunction|RandEps))
          (for _index_2 (range 0 (Math|Conversions|ToInteger(Byte) (/ (.y (Variables|Default|Getdims)) (Variables|Default|Geth))))
            (bind _eps_5 (CallFunction|RandEps))
            (for _index_3 (range 0 (Math|Conversions|ToInteger(Byte) (/ (.z (Variables|Default|Getdims)) (Variables|Default|Geth))))
              (bind _eps_6 (CallFunction|RandEps))
              (bind _output_get_3 (LocalVariables|Setp (Math|Vector|MakeVector (+ (* _index (Variables|Default|Geth)) _eps_4 (.x (Variables|Default|Getbmin))) (+ (* _index_2 (Variables|Default|Geth)) _eps_5 (.y (Variables|Default|Getbmin))) (+ (* _index_3 (Variables|Default|Geth)) _eps_6 (.z (Variables|Default|Getbmin))))))
              (bind _isinside (CallFunction|IsInside _output_get_3 (* (Variables|Default|Geth) 0.5)))
              (if _isinside
                (Utilities|Array|Add (Variables|Default|GetTetVerts) _output_get_3)))))))
    (:then_1
      (bind _output_get_4 (Variables|Default|Sets (* (Variables|Default|Getradius) 5.0)))
      (Utilities|Array|Add _tetverts (Math|Vector|MakeVector (* _output_get_4 -1.0) 0.0 (* _output_get_4 -1.0)))
      (Utilities|Array|Add _tetverts (Math|Vector|MakeVector _output_get_4 0.0 (* _output_get_4 -1.0)))
      (Utilities|Array|Add _tetverts (Math|Vector|MakeVector 0.0 _output_get_4 _output_get_4))
      (Utilities|Array|Add _tetverts (Math|Vector|MakeVector 0.0 (* _output_get_4 -1.0) _output_get_4)))))

(fn RandEps
  (bind _output_get (Variables|Default|Seteps 0.0001))
  (return (+ (* -1.0 _output_get) (* (Math|Random|RandomFloat) (Variables|Default|Geteps) 2.0))))

(fn IsInside
  (params (P :type Vector) (minDist :type Float%20%28double-precision%29))
  (LocalVariables|SetNumIn 0)
  (for _index (range 0 5)
    (Class|GeometryScriptLibraryMeshSpatial|FindNearestRayIntersectionwithMesh :TargetMesh (Variables|Default|GetTarget%20Mesh) :QueryBVH (Variables|Default|GetOutput%20BVH) :RayOrigin P :RayDirection (Utilities|Array|Get(acopy) (Variables|Default|Getdirs) _index) :Debug 0
      (:Found
        (Development|PrintString "jh")))))